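; Player-controlled claw that moves on the up and right input axes and grabs physics blocks.
; Grab press calls Grab, then runs a short vertical line trace at GrabLocation and attaches a simulating hit actor to the Claw's GrabLocation socket.
; Release detaches the block and reapplies its velocity as a velocity-change impulse, so it keeps its momentum.
; Grab, MoveUp and MoveRight are called here but defined outside this graph.
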(event EventBeginPlay)

(event Collision|EventActorBeginOverlap
  (params (OtherActor :type Actor%20Object%20Reference)))

(event EventTick
  (params (DeltaSeconds :type Float%20%28single-precision%29))
  (if (Variables|Default|GetIsGrabbed)
    _))

(event Input|ActionEvents|InputActionGrab
  (params (Key :type Key%20Structure))
  (bind _grablocation (Variables|Default|GetGrabLocation))
  (bind _returnvalue (Transformation|GetWorldLocation _grablocation))
  ;[1 1 1] Input Setup
  (:Pressed
    (Class|Claw|Grab)
    (bind (_outhit _returnvalue_2) (Collision|LineTraceForObjects _returnvalue (+ _returnvalue "0, 0,10.000000") (Utilities|Array|MakeArray "ObjectTypeQuery4") false 0 "None"))
    (if _returnvalue_2
      (if (Physics|IsSimulatingPhysics (.HitComponent (Collision|BreakHitResult _outhit)) "None")
        (bind _output_get (Variables|Default|SetGrabbedBlock (.HitActor (Collision|BreakHitResult _outhit))))
        (Transformation|AttachComponentToComponent _output_get (Variables|Default|GetClaw) "GrabLocation" "KeepWorld" "KeepWorld" "KeepWorld" true)
        (Variables|Default|SetIsGrabbed true))))
  (:Released
    (if (Variables|Default|GetIsGrabbed)
      (bind _asprimitive_component (Utilities|Casting|CastToPrimitiveComponent (Variables|/Script/Engine.Actor|GetRootComponent (Variables|Default|GetGrabbedBlock))))
      (bind _output_get_2 (Variables|Default|SetReleaseVelocity (Transformation|GetVelocity (Variables|Default|GetGrabbedBlock))))
      (Transformation|DetachFromComponent (Variables|/Script/Engine.Actor|GetRootComponent (Variables|Default|GetGrabbedBlock)) "KeepWorld" "KeepWorld" "KeepWorld" true)
      (Physics|AddImpulse _asprimitive_component _output_get_2 "None" true)
      (Variables|Default|SetIsGrabbed false)
      (Variables|Default|SetGrabbedBlock 0))))

(event Input|AxisEvents|InputAxisMoveUp
  (params (AxisValue :type Float%20%28single-precision%29))
  ;[1 1 1] Input Setup
  (Class|Claw|MoveUp AxisValue))

(event Input|AxisEvents|InputAxisMoveRight
  (params (AxisValue :type Float%20%28single-precision%29))
  ;[1 1 1] Input Setup
  (Class|Claw|MoveRight AxisValue))

(fn ConstructionScript)