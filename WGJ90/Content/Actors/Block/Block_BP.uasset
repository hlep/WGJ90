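; Block Blueprint actor that appears as either a green or red block, selected by its BlockColor variable.
; The construction script toggles visibility of the Block and RedBlock components to match the color; the Green case only shows Block and leaves RedBlock untouched.
; Every Tick resets the ParticleSystem's world rotation to zero, so the effect stays world-aligned however the actor rotates.
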(event EventBeginPlay)

(event Collision|EventActorBeginOverlap
  (params (OtherActor :type Actor%20Object%20Reference)))

(event EventTick
  (params (DeltaSeconds :type Float%20%28single-precision%29))
  (Transformation|SetWorldRotation (Variables|Default|GetParticleSystem) "0, 0, 0" false false))

(fn ConstructionScript
  (switch Utilities|FlowControl|Switch|SwitchonBlockEnum (Variables|Default|GetBlockColor)
    (:NewEnumerator0
      (Rendering|SetVisibility (Variables|Default|GetBlock) true false))
    (:NewEnumerator2
      (Rendering|SetVisibility (Variables|Default|GetBlock) false false)
      (Rendering|SetVisibility (Variables|Default|GetRedBlock) true false))))