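; Conveyor actor that carries Block_BP actors along its forward direction.
; Each tick it finds the Block_BP actors overlapping its Box and offsets those with a primitive root component by Speed scaled by delta time.
; Movement is a direct world offset without sweep or teleport, so it applies no forces and does not check for collisions along the way.
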(event EventBeginPlay)

(event Collision|EventActorBeginOverlap
  (params (OtherActor :type Actor%20Object%20Reference)))

(event EventTick
  (params (DeltaSeconds :type Float%20%28single-precision%29))
  (for _array_element (Collision|GetOverlappingActors (Variables|Default|GetBox) "/Game/Actors/Block/Block_BP.Block_BP_C" :!class /Script/Engine.PrimitiveComponent)
    (Utilities|Casting|CastToPrimitiveComponent (Variables|/Script/Engine.Actor|GetRootComponent _array_element))
    (Transformation|AddActorWorldOffset _array_element (* (Math|Conversions|ToVector(Float) (* DeltaSeconds (Variables|Default|GetSpeed))) (Math|Vector|GetForwardVector (Transformation|GetActorRotation))))))

(fn ConstructionScript)